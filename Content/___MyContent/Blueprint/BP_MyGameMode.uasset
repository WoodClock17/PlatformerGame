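; Game mode Blueprint that links to the level's game manager and provides setup for the game's UI widgets.
; On BeginPlay it caches the first BP_MyGameManager actor found in the world.
; CreateUI, which is not called within this Blueprint, creates the Abandon, Win, Lose and Health widgets, stores each on the manager and adds it to the viewport.
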(event EventBeginPlay
  (bind _outactors (Actor|GetAllActorsOfClass "/Game/___MyContent/Blueprint/BP_MyGameManager.BP_MyGameManager_C"))
  (Variables|Default|SetMy%20Game%20Manager (Utilities|Array|Get(acopy) _outactors)))

(event EventTick
  (params (DeltaSeconds :type Float%20%28single-precision%29)))

(fn ConstructionScript)

(fn CreateUI
  (bind _my_game_manager (CallFunction|GetMyGameManager))
  ;[1 1 1] Creates Abandon UI
  (bind _returnvalue (UserInterface|CreateWidget "/Game/___MyContent/UI/Widget_Abandon.Widget_Abandon_C"))
  (bind _output_get (Variables|/Game/___MyContent/Blueprint/BP_MyGameManager.BP_MyGameManager_C|SetWidgetAbandon _my_game_manager _returnvalue))
  (UserInterface|Viewport|AddtoViewport _output_get 0)
  ;[1 1 1] Creates Win UI
  (bind _returnvalue_2 (UserInterface|CreateWidget "/Game/___MyContent/UI/Widget_Win.Widget_Win_C"))
  (bind _output_get_2 (Variables|/Game/___MyContent/Blueprint/BP_MyGameManager.BP_MyGameManager_C|SetWidgetWin _my_game_manager _returnvalue_2))
  (UserInterface|Viewport|AddtoViewport _output_get_2 0)
  ;[1 1 1] Creates Lose UI
  (bind _returnvalue_3 (UserInterface|CreateWidget "/Game/___MyContent/UI/Widget_Lose.Widget_Lose_C"))
  (bind _output_get_3 (Variables|/Game/___MyContent/Blueprint/BP_MyGameManager.BP_MyGameManager_C|SetWidgetLose _my_game_manager _returnvalue_3))
  (UserInterface|Viewport|AddtoViewport _output_get_3 0)
  (bind _returnvalue_4 (UserInterface|CreateWidget "/Game/___MyContent/UI/Widget_Health.Widget_Health_C"))
  (bind _output_get_4 (Variables|/Game/___MyContent/Blueprint/BP_MyGameManager.BP_MyGameManager_C|SetWidgetHealth _my_game_manager _returnvalue_4))
  (UserInterface|Viewport|AddtoViewport _output_get_4 0))